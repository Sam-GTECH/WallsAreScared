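; BP_BasicMove is an actor that moves itself along the world X axis on a looping timeline, with Y and Z fixed.
; BeginPlay stores the start position and X limits at plus and minus MovingRange around it.
; Tick keeps the Move timeline playing, which restarts when finished.
; Its Alpha lerps between those absolute limits, and the result is added to the start X again, without sweep.
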(event `self.ReceiveBeginPlay`
  (bind _returnvalue_x (`KismetMathLibrary.BreakVector` (`self.K2_GetActorLocation`)))
  (set `self.MoveLimits` (`KismetMathLibrary.MakeVector2D` (- _returnvalue_x (`self.MovingRange`)) (+ _returnvalue_x (`self.MovingRange`))))
  (set `self.OrigPos` (`self.K2_GetActorLocation`)))

(event `self.ReceiveTick`
  (params (DeltaSeconds :type "Float (single-precision)"))
  (bind (_movelimits_x _movelimits_y) (`KismetMathLibrary.BreakVector2D` (`self.MoveLimits`)))
  (bind (_origpos_x _origpos_y _origpos_z) (`KismetMathLibrary.BreakVector` (`self.OrigPos`)))
  (bind (_direction _alpha) (`Timeline|Move` :!label _label)
    (:`Update`
      (`self.K2_SetActorLocation` (`KismetMathLibrary.MakeVector` (+ _origpos_x (`KismetMathLibrary.Lerp` _movelimits_x _movelimits_y _alpha)) _origpos_y _origpos_z)))
    (:`Finished`
      (goto _label :!via `PlayFromStart`))))

(fn `UserConstructionScript`)