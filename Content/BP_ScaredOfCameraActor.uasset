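; BP_ScaredOfCameraActor is a static mesh actor that drives an occlusion-masking material around the player when flagged as between camera and player.
; ActivateOcclusion sets that flag, forcing it off if any valid activator disallows masking, and prunes invalid activators.
; Tick grows or shrinks the dynamic material's clamped Radius at a set speed.
; It feeds in the player's position, frozen while the radius shrinks so the mask closes in place.
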(event `self.ReceiveBeginPlay`
  (bind _materialinstance (`self.MaterialInstance`))
  (bind _radiuslimit_x (`KismetMathLibrary.BreakVector2D` (`self.RadiusLimit`)))
  (`MaterialInstanceDynamic.SetVectorParameterValue` _materialinstance "None" (`KismetMathLibrary.Conv_VectorToLinearColor` (`self.K2_GetActorLocation` (`GameplayStatics.GetPlayerPawn` 0))))
  (`MaterialInstanceDynamic.SetScalarParameterValue` _materialinstance "Radius" _radiuslimit_x))

(event `self.ReceiveTick`
  (params (DeltaSeconds :type "Float (single-precision)"))
  (`|ExecutionSequence`
    (:`then_0`
      (`MaterialInstanceDynamic.SetScalarParameterValue` (`self.MaterialInstance`) "IsBetweenCamera" (`KismetMathLibrary.Conv_BoolToDouble` (or (`self.IsInbetweenCameraPlayer`) (`self.IsRadiusGoingDown`)))))
    (:`then_1`
      (bind _isradiusshrinking (`self.UpdateRadius` DeltaSeconds))
      (set `self.IsRadiusGoingDown` _isradiusshrinking))
    (:`then_3`
      (if (not (`self.IsRadiusGoingDown`))
        (`MaterialInstanceDynamic.SetVectorParameterValue` (`self.MaterialInstance`) "PlayerPos" (`KismetMathLibrary.Conv_VectorToLinearColor` (`self.K2_GetActorLocation` (`GameplayStatics.GetPlayerPawn` 0))))))))

(fn `ActivateOcclusion`
  (params (Toggle :type Boolean))
  (bind (_arrayindex _arrayelement) (`/Engine/EditorBlueprintResources/StandardMacros.ReverseForEachLoop` (`self.Activators`))
    (:`LoopBody`
      (`/Engine/EditorBlueprintResources/StandardMacros.IsValid` _arrayelement
        (:`Is Valid`
          (bind _allowed (`/Game/BP_OcclusionActivator.AllowOcclusionMasking` _arrayelement))
          (if (not _allowed)
            (set `self.IsInbetweenCameraPlayer` false)
            (return)))
        (:`Is Not Valid`
          (`KismetArrayLibrary.Array_RemoveItem` (`self.Activators`) _arrayelement))))
    (:`Completed`
      (set `self.IsInbetweenCameraPlayer` Toggle))))

(fn `UpdateRadius`
  (params (DeltaTime :type "Float (double-precision)"))
  (returns (IsRadiusShrinking :type Boolean))
  (locals (Radius :type "Float (double-precision)") (Allow :type Boolean :default true) (TempRadius :type "Float (double-precision)"))
  (bind (_radiuslimit_x _radiuslimit_y) (`KismetMathLibrary.BreakVector2D` (`self.RadiusLimit`)))
  (bind _radiuslimit_x_2 (`KismetMathLibrary.BreakVector2D` (`self.RadiusLimit`)))
  (bind _returnvalue (`MaterialInstanceDynamic.K2_GetScalarParameterValue` (`self.MaterialInstance`) "Radius"))
  (bind _output_get (set `local.Radius` _returnvalue))
  (set `local.TempRadius` _output_get)
  (if (`self.IsInbetweenCameraPlayer`)
    (set `local.Radius` (+ (`local.Radius`) (* (`local.DeltaTime`) (`self.RadiusSpeed`))))
    (else
      (set `local.Radius` (- (`local.Radius`) (* (`local.DeltaTime`) (`self.RadiusSpeed`))))))
  (`MaterialInstanceDynamic.SetScalarParameterValue` (`self.MaterialInstance`) "Radius" (`KismetMathLibrary.FClamp` (`local.Radius`) _radiuslimit_x _radiuslimit_y))
  (return (and (> (`local.Radius`) _radiuslimit_x_2) (< (`local.Radius`) (`local.TempRadius`)))))

(fn `UserConstructionScript`
  (bind _returnvalue (`PrimitiveComponent.CreateDynamicMaterialInstance` (`self.StaticMesh`) 0 "/Game/MI_ScaredOfCamera.MI_ScaredOfCamera" "None"))
  (bind _output_get (set `self.MaterialInstance` _returnvalue))
  (`MaterialInstanceDynamic.SetTextureParameterValue` _output_get "Texture" (`self.Texture`)))