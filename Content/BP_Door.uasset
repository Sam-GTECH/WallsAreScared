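; BP_Door is a door the player toggles open and closed with the E key while a BP_ThirdPersonCharacter overlaps the actor.
; Overlap events track whether that character is in range, and the key press flips the open flag only then.
; Tick plays or reverses a timeline from that flag, lerping the door's world Z between its BeginPlay height and that height plus an offset.
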(event `self.ReceiveBeginPlay`
  (bind (_returnvalue_x _returnvalue_y _returnvalue_z) (`KismetMathLibrary.BreakVector` (`SceneComponent.K2_GetComponentLocation` (`self.Door`))))
  (set `self.DefaultZ` _returnvalue_z))

(event `self.ReceiveTick`
  (params (DeltaSeconds :type "Float (single-precision)"))
  (bind (_returnvalue_x _returnvalue_y) (`KismetMathLibrary.BreakVector` (`SceneComponent.K2_GetComponentLocation` (`self.Door`))))
  (if (`self.IsDoorOpened`)
    (bind (_direction _lerpalpha) (`Timeline|DoorAnimation` :!label _label)
      (:`Update`
        (`SceneComponent.K2_SetWorldLocation` (`self.Door`) (`KismetMathLibrary.MakeVector` _returnvalue_x _returnvalue_y (`KismetMathLibrary.Lerp` (`self.DefaultZ`) (+ (`self.DefaultZ`) (`self.OpenZ`)) _lerpalpha)) false false)))
    (else
      (goto _label :!via `Reverse`))))

(event `self.ReceiveActorBeginOverlap`
  (params (OtherActor :type "Actor Object Reference"))
  (if (`GameplayStatics.ObjectIsA` OtherActor "/Game/ThirdPerson/Blueprints/BP_ThirdPersonCharacter.BP_ThirdPersonCharacter_C")
    (set `self.IsPlayerOverlapping` true)))

(event `self.ReceiveActorEndOverlap`
  (params (OtherActor :type "Actor Object Reference"))
  (if (`GameplayStatics.ObjectIsA` OtherActor "/Game/ThirdPerson/Blueprints/BP_ThirdPersonCharacter.BP_ThirdPersonCharacter_C")
    (set `self.IsPlayerOverlapping` false)))

(event `Key|E`
  (params (Key :type "Key Structure"))
  (:`Pressed`
    (if (`self.IsPlayerOverlapping`)
      (set `self.IsDoorOpened` (not (`self.IsDoorOpened`))))))

(fn `UserConstructionScript`)